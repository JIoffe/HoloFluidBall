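; BP_SpawnFluidBallButton is a button Blueprint that spawns a BP_HoloFluidBall in front of the player's view.
; On each ButtonComponent press it destroys the ball it previously spawned, then creates a new one a fixed distance along the camera's forward vector.
; It stores the new ball in FluidBallActor, so each button keeps at most one ball, owned and instigated by the player pawn.
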(event `self.ButtonComponent.OnButtonPressed`
  (params (Button :type "UxtPressableButtonComponent Object Reference") (Pointer :type "UxtPointerComponent Object Reference"))
  (bind _returnvalue (`GameplayStatics.GetPlayerPawn` 0))
  (bind _returnvalue_2 (`GameplayStatics.GetPlayerCameraManager` 0))
  (bind _fluidballactor (`self.FluidBallActor`))
  (`|ExecutionSequence`
    (:`then_0`
      (if (`KismetSystemLibrary.IsValid` _fluidballactor)
        (`self.K2_DestroyActor` _fluidballactor)
        (set `self.FluidBallActor` null)))
    (:`then_1`
      (bind _returnvalue_3 (`|SpawnActorFromClass` "/Game/Blueprints/BP_HoloFluidBall.BP_HoloFluidBall_C" (`KismetMathLibrary.MakeTransform` (+ (* (`self.GetActorForwardVector` _returnvalue_2) 200.0) (`PlayerCameraManager.GetCameraLocation` _returnvalue_2))) "Undefined" "OverrideRootScale" _returnvalue _returnvalue))
      (set `self.FluidBallActor` _returnvalue_3))))

(fn `UserConstructionScript`)