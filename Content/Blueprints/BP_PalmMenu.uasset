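; BP_PalmMenu is a hand menu built on Mixed Reality UX Tools that appears while the palm-up constraint is active.
; Activation shows the UI element and spawns a hand interaction actor set to AnyHand, owned by the player pawn.
; Deactivation hides the UI and destroys that actor, so this interaction actor exists only while the menu is up.
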(event `self.UxtPalmUpConstraint.OnConstraintActivated`
  (bind _returnvalue (`GameplayStatics.GetPlayerPawn` 0))
  (`UxtUIElementComponent.SetUIVisibility` (`self.UxtUIElement`) "Show")
  (bind _returnvalue_2 (`|SpawnActorFromClass` "/Script/UXTools.UxtHandInteractionActor" (`KismetMathLibrary.MakeTransform` (0.0 0.0 0.0)) "Undefined" "OverrideRootScale" _returnvalue false "AnyHand" _returnvalue))
  (set `self.HandInteractionActor` _returnvalue_2))

(event `self.UxtPalmUpConstraint.OnConstraintDeactivated`
  (bind _handinteractionactor (`self.HandInteractionActor`))
  (`UxtUIElementComponent.SetUIVisibility` (`self.UxtUIElement`) "Hide")
  (if (`KismetSystemLibrary.IsValid` _handinteractionactor)
    (`self.K2_DestroyActor` _handinteractionactor)
    (set `self.HandInteractionActor` null)))

(fn `UserConstructionScript`)