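; BP_HoloFluidBall is a camera-facing holographic fluid ball that reacts to the player's tracked hands.
; Tick billboards the actor and writes index, thumb and little fingertip positions from both hands into six node parameters on a dynamic material.
; Each node packs world position in RGB and tip radius in alpha; an untracked hand's nodes collapse to the mesh location.
; The MaximumRange mesh scaling is unconnected, so it never runs.
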(event `self.ReceiveBeginPlay`
  (bind _mesh (`self.Mesh`))
  (bind _returnvalue (`PrimitiveComponent.CreateDynamicMaterialInstance` _mesh 0 (`PrimitiveComponent.GetMaterial` _mesh 0) "None"))
  (set `self.FluidMaterial` _returnvalue))

(event `self.ReceiveTick`
  (params (DeltaSeconds :type "Float (single-precision)"))
  (bind _returnvalue (`GameplayStatics.GetPlayerCameraManager` 0))
  (bind _fluidmaterial (`self.FluidMaterial`))
  (bind _fluidmaterial_2 (`self.FluidMaterial`))
  (bind (_returnvalue_x _returnvalue_y _returnvalue_z) (`KismetMathLibrary.BreakVector` (`SceneComponent.K2_GetComponentLocation` (`self.Mesh`))))
  (bind (_returnvalue_x_2 _returnvalue_y_2 _returnvalue_z_2) (`KismetMathLibrary.BreakVector` (`SceneComponent.K2_GetComponentLocation` (`self.Mesh`))))
  (bind _linearcolor (make `LinearColor` _returnvalue_x_2 _returnvalue_y_2 _returnvalue_z_2))
  (bind _linearcolor_2 (make `LinearColor` _returnvalue_x _returnvalue_y _returnvalue_z))
  (`|ExecutionSequence`
    (:`then_0`
      ;[1 1 1] Billboard against camera
      (`self.K2_SetActorRotation` (`KismetMathLibrary.MakeRotFromXZ` (- (`PlayerCameraManager.GetCameraLocation` _returnvalue) (`self.K2_GetActorLocation`)) (`self.GetActorUpVector` _returnvalue))))
    (:`then_1`
      ;[1 1 1] Right Hand
      (bind _motioncontrollerdata (`HeadMountedDisplayFunctionLibrary.GetMotionControllerData` null "Right"))
      (bind (_bvalid _devicename _applicationinstanceid _devicevisualtype _handindex _trackingstatus _gripposition _griprotation _aimposition _aimrotation _handkeypositions) (break `XRMotionControllerData` _motioncontrollerdata))
      (if (and _bvalid (`|EnumEquality` _devicevisualtype "Hand") (> (`KismetArrayLibrary.Array_Length` _handkeypositions) 0))
        (bind (_output_x _output_y _output_z) (`KismetMathLibrary.BreakVector` (`|GetArrayItem` _handkeypositions (`KismetMathLibrary.Conv_ByteToInt` (enumliteral `EHandKeypoint` "IndexTip")))))
        (`MaterialInstanceDynamic.SetVectorParameterValue` _fluidmaterial_2 "Node1" (make `LinearColor` _output_x _output_y _output_z (`self.NoduleTipRadius`)))
        (bind (_output_x_2 _output_y_2 _output_z_2) (`KismetMathLibrary.BreakVector` (`|GetArrayItem` _handkeypositions (`KismetMathLibrary.Conv_ByteToInt` (enumliteral `EHandKeypoint` "ThumbTip")))))
        (`MaterialInstanceDynamic.SetVectorParameterValue` _fluidmaterial_2 "Node2" (make `LinearColor` _output_x_2 _output_y_2 _output_z_2 (`self.NoduleTipRadius`)))
        (bind (_output_x_3 _output_y_3 _output_z_3) (`KismetMathLibrary.BreakVector` (`|GetArrayItem` _handkeypositions (`KismetMathLibrary.Conv_ByteToInt` (enumliteral `EHandKeypoint` "LittleTip")))))
        (`MaterialInstanceDynamic.SetVectorParameterValue` _fluidmaterial_2 "Node3" (make `LinearColor` _output_x_3 _output_y_3 _output_z_3 (`self.NoduleTipRadius`)))
        (else
          ;;[1 1 1] Zero out nodules if hands are not visible
          (`MaterialInstanceDynamic.SetVectorParameterValue` _fluidmaterial_2 "Node1" _linearcolor_2)
          (`MaterialInstanceDynamic.SetVectorParameterValue` _fluidmaterial_2 "Node2" _linearcolor_2)
          (`MaterialInstanceDynamic.SetVectorParameterValue` _fluidmaterial_2 "Node3" _linearcolor_2))))
    (:`then_2`
      ;[1 1 1] Right Hand
      (bind _motioncontrollerdata_2 (`HeadMountedDisplayFunctionLibrary.GetMotionControllerData` null "Left"))
      (bind (_bvalid_2 _devicename_2 _applicationinstanceid_2 _devicevisualtype_2 _handindex_2 _trackingstatus_2 _gripposition_2 _griprotation_2 _aimposition_2 _aimrotation_2 _handkeypositions_2) (break `XRMotionControllerData` _motioncontrollerdata_2))
      (if (and _bvalid_2 (`|EnumEquality` _devicevisualtype_2 "Hand") (> (`KismetArrayLibrary.Array_Length` _handkeypositions_2) 0))
        (bind (_output_x_4 _output_y_4 _output_z_4) (`KismetMathLibrary.BreakVector` (`|GetArrayItem` _handkeypositions_2 (`KismetMathLibrary.Conv_ByteToInt` (enumliteral `EHandKeypoint` "IndexTip")))))
        (`MaterialInstanceDynamic.SetVectorParameterValue` _fluidmaterial "Node4" (make `LinearColor` _output_x_4 _output_y_4 _output_z_4 (`self.NoduleTipRadius`)))
        (bind (_output_x_5 _output_y_5 _output_z_5) (`KismetMathLibrary.BreakVector` (`|GetArrayItem` _handkeypositions_2 (`KismetMathLibrary.Conv_ByteToInt` (enumliteral `EHandKeypoint` "ThumbTip")))))
        (`MaterialInstanceDynamic.SetVectorParameterValue` _fluidmaterial "Node5" (make `LinearColor` _output_x_5 _output_y_5 _output_z_5 (`self.NoduleTipRadius`)))
        (bind (_output_x_6 _output_y_6 _output_z_6) (`KismetMathLibrary.BreakVector` (`|GetArrayItem` _handkeypositions_2 (`KismetMathLibrary.Conv_ByteToInt` (enumliteral `EHandKeypoint` "LittleTip")))))
        (`MaterialInstanceDynamic.SetVectorParameterValue` _fluidmaterial "Node6" (make `LinearColor` _output_x_6 _output_y_6 _output_z_6 (`self.NoduleTipRadius`)))
        (else
          ;;[1 1 1] Zero out nodules if hands are not visible
          (`MaterialInstanceDynamic.SetVectorParameterValue` _fluidmaterial "Node4" _linearcolor)
          (`MaterialInstanceDynamic.SetVectorParameterValue` _fluidmaterial "Node5" _linearcolor)
          (`MaterialInstanceDynamic.SetVectorParameterValue` _fluidmaterial "Node6" _linearcolor))))))

(fn `UserConstructionScript`)